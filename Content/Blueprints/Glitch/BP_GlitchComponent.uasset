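; Player component for the first-person glitch ability, handling aiming, double-tap dash input and feedback.
; Tick traces from the camera to classify glitch targets and broadcast changes, while a separate trace sets the glitch direction toward targets or through nearby walls.
; Glitch and dash events swap the body material, toggle the crosshair and spawn state-specific particles and sounds.
; Particle effects are hurried along by advancing their simulation rather than changing playback rate.
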(event EventBeginPlay
  ;[1 0.03156 0] Begin play
  (bind _asbp_first_person_character_glitch (Utilities|Casting|CastToBP_FirstPersonCharacter_Glitch (Components|GetOwner)))
  (bind _playermesh (Default|GetPlayerMesh _asbp_first_person_character_glitch))
  (bind _output_get (Variables|Default|SetPlayerMesh _playermesh))
  (bind _returnvalue (Rendering|Material|CreateDynamicMaterialInstance _output_get 0 "/Game/Materials/M_FirstPersonBody.M_FirstPersonBody" "None" :!class /Script/Engine.PrimitiveComponent)) ; Set normal material here
  (Variables|Default|SetDynamicMaterial _returnvalue)
  (bind _returnvalue_2 (UserInterface|CreateWidget "/Game/Blueprints/Glitch/WBP_GlitchCrosshairWidget.WBP_GlitchCrosshairWidget_C" (Game|GetPlayerController 0)))
  (Variables|Default|SetCrosshairWidget _returnvalue_2))

(event EventOnDashStart
  ;[0.6903 1 0.7818] Spawn Particles / VFX
  (Widget|RemovefromParent (Variables|Default|GetCrosshairWidget))
  (switch Utilities|FlowControl|Switch|SwitchonGlitchState (Variables|Default|GetCurrentGlitchState)
    (:Upward
      ;;[0.2399 1 0] Upward Dash Particles
      (bind _returnvalue (Niagara|SpawnSystemAttached "/Game/VFX/Glitch/FXS_GlitchParticles_Dash_Upward.FXS_GlitchParticles_Dash_Upward" (Variables|Default|GetCollider) "None" "30.000000, 0,0.000000" "0, 0, 0" "KeepRelativeOffset" true))
      (bind _output_get (Variables|Default|SetCurrentDashParticles _returnvalue))
      (if (Utilities|Enum|NotEqual(Enum) (Variables|Default|GetCurrentTargetType) "NewEnumerator0")
        (CallFunction|SetParticlePlaybackSpeed _output_get 4.0)
        (else
          (Class|FMODBlueprintStatics|PlayEvent2D "/Game/FMOD/Events/player/glitchdash_upward.glitchdash_upward"))))
    (:Forwards
      ;;[0 1 0.656] Forward Dash Particles
      (bind _returnvalue_2 (Niagara|SpawnSystemAttached "/Game/VFX/Glitch/FXS_GlitchParticles_Dash_Short_Green.FXS_GlitchParticles_Dash_Short_Green" (Variables|Default|GetCameraComponent) "None" "320.000000, 0, 0" "0, 0, 0" "KeepRelativeOffset" true))
      (bind _output_get_2 (Variables|Default|SetCurrentDashParticles _returnvalue_2))
      (Effects|Components|ParticleSystem|SetVectorParameter _output_get_2 "Velocity" (* (Math|Vector|GetForwardVector (Variables|Default|GetCameraComponent)) -1e+03))
      (Effects|Components|ParticleSystem|SetVectorParameter _output_get_2 "CameraPosition" (Transformation|GetWorldLocation (Variables|Default|GetCameraComponent))))
    (:TowardTarget
      ;;[0 0.6366 1] Target glitch particles
      (bind _particlespawnlocation (CallFunction|GetParticleSpawnLocation 3e+02 559.0))
      (Utilities|FlowControl|Delay (Math|Float|Lerp 0.0 0.3 (Math|Float|Clamp(Float) (/ (Math|Vector|VectorLength (- (Variables|Default|GetGlitchTargetLocation) (Transformation|GetWorldLocation (Variables|Default|GetCameraComponent)))) 5e+03))))
      (bind _returnvalue_3 (Niagara|SpawnSystemAttached "/Game/VFX/Glitch/FXS_GlitchParticles_Dash.FXS_GlitchParticles_Dash" (Variables|Default|GetCameraComponent) "None" _particlespawnlocation "0, 0, 0" "KeepWorldPosition" true))
      (bind _output_get_3 (Variables|Default|SetCurrentDashParticles _returnvalue_3))
      (Effects|Components|ParticleSystem|SetVectorParameter _output_get_3 "Velocity" (* (Math|Vector|Normalize (- (Variables|Default|GetGlitchTargetLocation) (Transformation|GetWorldLocation (Variables|Default|GetCameraComponent)))) -7.8e+02))
      (Class|FMODBlueprintStatics|PlayEvent2D "/Game/FMOD/Events/player/glitchdash_forward.glitchdash_forward"))
    (:GlitchThrough
      ;;[0 1 0.7415] Glitch through wall
      (bind _returnvalue_4 (Niagara|SpawnSystemAttached "/Game/VFX/Glitch/FXS_GlitchParticles_Dash.FXS_GlitchParticles_Dash" (Variables|Default|GetCameraComponent) "None" "300.000000, 0, 0" "0, 0, 0" "KeepRelativeOffset" true))
      (Variables|Default|SetCurrentDashParticles _returnvalue_4)
      (Class|FMODBlueprintStatics|PlayEvent2D "/Game/FMOD/Events/player/glitchdash_forward.glitchdash_forward"))))

(event EventTick
  (params (DeltaSeconds :type Float%20%28single-precision%29))
  ;[1 1 1] TODO: Move to c++
  (CallFunction|UpdateGlitchableTarget))

(event EventOnPassingThroughObject
  ;[0.6861 0.5526 1] Boost playback speed of particles after passing through object
  (bind _currentdashparticles (Variables|Default|GetCurrentDashParticles)
    (:then
      (CallFunction|SetParticlePlaybackSpeed _currentdashparticles 5e+01))
    (:else)))

(event EventOnGlitchingStart
  ;[0.2719 1 0.1332] On Glitching Start/End
  (Rendering|Material|SetMaterial (Variables|Default|GetPlayerMesh) 0 "/Game/Materials/M_GlitchBody.M_GlitchBody") ; Set glitch material here
  (bind _returnvalue (Niagara|SpawnSystemAttached "/Game/VFX/Glitch/FXS_GlitchParticles.FXS_GlitchParticles" (Variables|Default|GetCollider) "None" "50.000000, 0,50.000000" "0, 0, 0" "KeepRelativeOffset" true))
  (bind _currentstaticparticles (Variables|Default|GetCurrentStaticParticles)
    (:then
      (Components|Activation|Deactivate _currentstaticparticles))
    (:else
      _))
  (Variables|Default|SetCurrentStaticParticles _returnvalue)
  (UserInterface|Viewport|AddtoViewport (Variables|Default|GetCrosshairWidget) 0))

(event EventOnGlitchingEnd
  (bind _playermesh (Variables|Default|GetPlayerMesh))
  ;[0.2719 1 0.1332] On Glitching Start/End
  (Rendering|Material|SetMaterial _playermesh 0 (Variables|Default|GetDynamicMaterial))
  (Collision|SetCollisionResponsetoAllChannels _playermesh "ECR_Block")
  (bind _currentdashparticles (Variables|Default|GetCurrentDashParticles)
    (:then
      (CallFunction|SetParticlePlaybackSpeed _currentdashparticles 1e+02))
    (:else
      _))
  (Widget|RemovefromParent (Variables|Default|GetCrosshairWidget))
  (Variables|Default|SetCurrentTargetType "NewEnumerator3")
  (bind _currentstaticparticles (Variables|Default|GetCurrentStaticParticles)
    (:then
      (Components|Activation|Deactivate _currentstaticparticles))
    (:else)))

(fn SetParticlePlaybackSpeed
  (params (ParticleSystem :type Niagara%20Component%20Object%20Reference) (TimeMultiplier :type Float%20%28single-precision%29))
  (bind _returnvalue (Utilities|Time|GetWorldDeltaSeconds))
  (if (Utilities|IsValid ParticleSystem)
    (Class|NiagaraComponent|AdvanceSimulationbyTime ParticleSystem (* _returnvalue TimeMultiplier) _returnvalue)
    (else
      (Development|PrintString "NOT VALID PARTICLE SYSTEM" true true "(R=1.000000,G=0.000000,B=0.021455,A=1.000000)"))))

(fn SetGlitchTargetLocation
  (bind _cameracomponent (Variables|Default|GetCameraComponent))
  (bind _returnvalue (Transformation|GetSocketLocation _cameracomponent "None"))
  ;[0.7321 0.7111 1] Line trace in the direction of the camera
  (bind (_outhit _returnvalue_2) (Collision|LineTraceForObjects _returnvalue (+ _returnvalue (* (Math|Vector|GetForwardVector (Variables|Default|GetCameraComponent)) 5e+03)) (LocalVariables|GetGlitchTarget) false 0 "None"))
  (if _returnvalue_2
    (switch Utilities|FlowControl|Switch|SwitchonECollisionChannel (Collision|GetCollisionObjectType (.HitComponent (Collision|BreakHitResult _outhit)))
      (:ECC_GameTraceChannel1
        ;[0.5795 1 0.2586] Check if close enough to glitchable wall
        (if (< (.Distance (Collision|BreakHitResult _outhit)) (Variables|Default|GetGlitchThroughWallMaxDistance))
          (Variables|Default|SetCurrentTargetType "NewEnumerator0")
          (Class|GlitchComponent|SetGlitchDirection (Math|Conversions|ToInteger(Byte) (Utilities|Enum|LiteralenumGlitchState "GlitchThrough")) "0, 0, 0")))
      (:ECC_GameTraceChannel2
        ;[1 1 1] Get Location of impact, add Z offset
        (LocalVariables|SetTargetLocation (+ (.ImpactPoint (Collision|BreakHitResult _outhit)) (* (LocalVariables|GetZOffsetVector) (Math|Float|Clamp(Float) (.Z (Math|Vector|BreakVector (.Normal (Collision|BreakHitResult _outhit)))))) (* (Math|Vector|GetForwardVector (Variables|Default|GetCameraComponent)) -1e+02)))
        (Variables|Default|SetCurrentTargetType "NewEnumerator1")
        (Class|GlitchComponent|SetGlitchDirection (Math|Conversions|ToInteger(Byte) (Utilities|Enum|LiteralenumGlitchState "TowardTarget")) (LocalVariables|GetTargetLocation))
        (Rendering|Debug|DrawDebugCircle "0, 0, 0" 5e+01 12 "(R=0.057249,G=1.000000,B=0.000000,A=1.000000)" 2.0 0.1 "0.000000,1.000000,0.000000" "0.000000,0.000000,1.000000")))))

(fn CheckGlitchingDirection
  (params (Direction :type Vector) (Distance :type Float%20%28single-precision%29))
  (bind _returnvalue (Components|GetOwner))
  (bind _rootcomponent (Variables|/Script/Engine.Actor|GetRootComponent _returnvalue))
  (bind _returnvalue_2 (Transformation|GetWorldLocation _rootcomponent))
  (bind _returnvalue_3 (Collision|LineTraceForObjects _returnvalue_2 (+ (* Direction Distance) _returnvalue_2) (LocalVariables|GetObjectTypes) false 0 "ForDuration" true "(R=0.132879,G=1.000000,B=0.000000,A=1.000000)" "(R=0.000000,G=1.000000,B=0.000000,A=1.000000)" 0.5))
  (return _returnvalue_3))

(fn GetParticleSpawnLocation
  (params (MinDistance :type Float%20%28single-precision%29) (MaxDistance :type Float%20%28single-precision%29))
  (bind _cameracomponent (Variables|Default|GetCameraComponent))
  (bind _returnvalue (Math|Vector|GetForwardVector _cameracomponent))
  (bind _canglitch (CallFunction|CheckGlitchingDirection _returnvalue 5e+02))
  (if _canglitch
    (Variables|Default|SetParticleDistance MinDistance)
    (else
      (Variables|Default|SetParticleDistance MaxDistance)))
  (return (+ (* _returnvalue (Variables|Default|GetParticleDistance)) (Transformation|GetWorldLocation _cameracomponent))))

(fn HandleForwardInput
  (if (and (< (- (Actor|GetGameTimeSinceCreation (Components|GetOwner)) (Variables|Default|GetTimeOfLastForwardInput)) (Variables|Default|GetMaxTapInterval)) (not (Variables|Default|GetbIsOnCooldown)))
    (Class|GlitchComponent|StartShortDash 3)
    (CameraShakes|StartCameraShake (Game|GetPlayerCameraManager 0) "/Game/Blueprints/Glitch/CS_Dash.CS_Dash_C" 1e+01 "CameraLocal" "0, 0, 0")
    (bind _currentstaticparticles (Variables|Default|GetCurrentStaticParticles)
      (:then
        (Components|Activation|Deactivate _currentstaticparticles))
      (:else
        _)))
  (Variables|Default|SetTimeOfLastForwardInput (Actor|GetGameTimeSinceCreation (Components|GetOwner))))

(fn UpdateGlitchableTarget
  (bind _cameracomponent (Variables|Default|GetCameraComponent))
  (bind _returnvalue (Transformation|GetSocketLocation _cameracomponent "None"))
  ;[0.7321 0.7111 1] Line trace in the direction of the camera
  (bind (_outhit _returnvalue_2) (Collision|LineTraceForObjects _returnvalue (+ _returnvalue (* (Math|Vector|GetForwardVector (Variables|Default|GetCameraComponent)) 5e+03)) (LocalVariables|GetGlitchTarget) false 0 "None"))
  (if _returnvalue_2
    (switch Utilities|FlowControl|Switch|SwitchonECollisionChannel (Collision|GetCollisionObjectType (.HitComponent (Collision|BreakHitResult _outhit)))
      (:ECC_WorldStatic
        (if (not (Utilities|Enum|Equal(Enum) (Variables|Default|GetCurrentTargetType) "NewEnumerator3")) :!label _label
          (Variables|Default|SetCurrentTargetType "NewEnumerator3")
          (Default|CallTargetTypeChanged (Variables|Default|GetCurrentTargetType) :!label _label_2)))
      (:ECC_WorldDynamic
        (goto _label))
      (:ECC_Pawn
        (goto _label))
      (:ECC_Visibility
        (goto _label))
      (:ECC_Camera
        (goto _label))
      (:ECC_PhysicsBody
        (goto _label))
      (:ECC_Vehicle
        (goto _label))
      (:ECC_Destructible
        (goto _label))
      (:ECC_GameTraceChannel1
        (if (< (.Distance (Collision|BreakHitResult _outhit)) (Variables|Default|GetGlitchThroughWallMaxDistance))
          (if (not (Utilities|Enum|Equal(Enum) (Variables|Default|GetCurrentTargetType) "NewEnumerator0"))
            (Variables|Default|SetCurrentTargetType "NewEnumerator0")
            (goto _label_2))
          (elif (not (Utilities|Enum|Equal(Enum) (Variables|Default|GetCurrentTargetType) "NewEnumerator2"))
            (Variables|Default|SetCurrentTargetType "NewEnumerator2")
            (goto _label_2))))
      (:ECC_GameTraceChannel2
        (if (not (Utilities|Enum|Equal(Enum) (Variables|Default|GetCurrentTargetType) "NewEnumerator1"))
          (Variables|Default|SetCurrentTargetType "NewEnumerator1")
          (goto _label_2)))
      (:ECC_GameTraceChannel3
        (goto _label)))
    (else
      (goto _label))))

(fn HandleUpwardInput
  (if (and (< (- (Actor|GetGameTimeSinceCreation (Components|GetOwner)) (Variables|Default|GetTimeOfLastUpwardInput)) (Variables|Default|GetMaxTapInterval)) (not (Variables|Default|GetbIsOnCooldown)))
    (Class|GlitchComponent|StartShortDash 2)
    (CameraShakes|StartCameraShake (Game|GetPlayerCameraManager 0) "/Game/Blueprints/Glitch/CS_Dash.CS_Dash_C" 1e+01 "CameraLocal" "0, 0, 0")
    (bind _currentstaticparticles (Variables|Default|GetCurrentStaticParticles)
      (:then
        (Components|Activation|Deactivate _currentstaticparticles))
      (:else
        _)))
  (Variables|Default|SetTimeOfLastUpwardInput (Actor|GetGameTimeSinceCreation (Components|GetOwner))))

(fn OnTargetTypeChanged
  (params (NewTargetType :type TargetType%20Enum :default "NewEnumerator0"))
  ;[1 1 1] Only made to copy delegate input
)