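; Portal door paired with a TeleportTarget door, showing a live view through it and teleporting the first-person player on overlap.
; Each tick positions the target's scene capture from the player camera's relative transform, with construction cross-wiring render targets into portal materials.
; Teleporting preserves relative view and velocity, briefly disables the destination portal and flashes post-process.
; A temporary trigger timeline swings both doors open, pending proper character interaction.
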(event OnComponentEndOverlap(Portal)
  (params (OverlappedComponent :type Primitive%20Component%20Object%20Reference) (OtherActor :type Actor%20Object%20Reference) (OtherComp :type Primitive%20Component%20Object%20Reference) (OtherBodyIndex :type Integer))
  ;[1 1 1] Reactivate Portal
  (CallFunction|ShowPortal))

(event OnComponentBeginOverlap(DoorTrigger)
  (params (OverlappedComponent :type Primitive%20Component%20Object%20Reference) (OtherActor :type Actor%20Object%20Reference) (OtherComp :type Primitive%20Component%20Object%20Reference) (OtherBodyIndex :type Integer) (bFromSweep :type Boolean) (SweepResult :type Hit%20Result%20Structure%20%28by%20ref%29))
  ;[1 1 1] Open/Close Door -  REMOVE THIS AFTER PROPPER CHARACTER INTERACTION IS DONE
  (if (Variables|Default|GetCanPort)
    (bind _door (Timeline|Timeline_0 Play)
      (:Update
        (Transformation|SetRelativeRotation (Variables|Default|GetSM_PortalDoor) (Math|Rotator|MakeRotator 0.0 0.0 (* _door -1.4e+02)) false false)
        (Transformation|SetRelativeRotation (Variables|BP_PortalDoor_C|GetSM_PortalDoor (Variables|Default|GetTeleport%20Target)) (Math|Rotator|MakeRotator 0.0 0.0 (* _door -1.4e+02)) false false)))))

(event OnComponentEndOverlap(DoorTrigger)
  (params (OverlappedComponent :type Primitive%20Component%20Object%20Reference) (OtherActor :type Actor%20Object%20Reference) (OtherComp :type Primitive%20Component%20Object%20Reference) (OtherBodyIndex :type Integer))
  ;[1 1 1] Open/Close Door -  REMOVE THIS AFTER PROPPER CHARACTER INTERACTION IS DONE
  (Utilities|FlowControl|Delay 0.2)
  (bind _door (Timeline|Timeline_0 Reverse)
    (:Update
      (Transformation|SetRelativeRotation (Variables|Default|GetSM_PortalDoor) (Math|Rotator|MakeRotator 0.0 0.0 (* _door -1.4e+02)) false false)
      (Transformation|SetRelativeRotation (Variables|BP_PortalDoor_C|GetSM_PortalDoor (Variables|Default|GetTeleport%20Target)) (Math|Rotator|MakeRotator 0.0 0.0 (* _door -1.4e+02)) false false))))

(event OnComponentBeginOverlap(Portal)
  (params (OverlappedComponent :type Primitive%20Component%20Object%20Reference) (OtherActor :type Actor%20Object%20Reference) (OtherComp :type Primitive%20Component%20Object%20Reference) (OtherBodyIndex :type Integer) (bFromSweep :type Boolean) (SweepResult :type Hit%20Result%20Structure%20%28by%20ref%29))
  (bind _postprocess (Variables|Default|GetPostProcess))
  ;[1 1 1] Teleport Player
  (Utilities|IsValid (Variables|Default|GetTeleport%20Target)
    (:Is%20Valid
      (if (Variables|Default|GetCanPort)
        (CallFunction|HidePortal (Variables|Default|GetTeleport%20Target))
        (Utilities|FlowControl|Delay 0.05)
        (CallFunction|TeleportPlayer (Variables|Default|GetPlayer))
        (Rendering|SetVisibility _postprocess true false)
        (Utilities|FlowControl|Delay 0.25)
        (Rendering|SetVisibility _postprocess false false)))))

(event Custom|ShowPortal
  ;[1 1 1] Show/Hide Portal Functions
  (Utilities|FlowControl|Delay 1.0)
  (Components|Activation|SetActive (Variables|Default|GetPortal) true true)
  (Variables|Default|SetCanPort true))

(event Custom|HidePortal
  ;[1 1 1] Show/Hide Portal Functions
  (Components|Activation|Deactivate (Variables|Default|GetPortal))
  (Variables|Default|SetCanPort false))

(event Custom|TeleportPlayerEvent
  (params (Location :type Vector) (Rotation :type Rotator))
  ;[1 1 1] Telport Player
)

(event EventTick
  (params (DeltaSeconds :type Float%20%28single-precision%29))
  (bind _returnvalue (Game|GetPlayerCameraManager 0))
  (bind _portalviewbackface (Variables|Default|GetPortalViewBackface))
  (bind _returnvalue_2 (Transformation|GetWorldTransform _portalviewbackface))
  (bind _transformcomponent (Variables|/Script/Engine.PlayerCameraManager|GetTransformComponent _returnvalue))
  (bind _returnvalue_3 (Transformation|GetWorldTransform _transformcomponent))
  (bind _returnvalue_4 (Class|KismetMathLibrary|ConvertTransformtoRelative _returnvalue_2 _returnvalue_3))
  ;[1 1 1] Scene capture position relative to player
  (Utilities|FlowControl|Sequence
    (:then_0
      (Transformation|SetRelativeLocationAndRotation (Variables|BP_PortalDoor_C|GetPortalViewCapture (Variables|Default|GetTeleport%20Target)) (.location _returnvalue_4) (.rotation _returnvalue_4) false false))))

(event EventBeginPlay
  ;[1 1 1] Set Player
  (bind _asbp_first_person_character_glitch (Utilities|Casting|CastToBP_FirstPersonCharacter_Glitch (Game|Player|GetPlayerPawn 0)))
  (Variables|Default|SetPlayer _asbp_first_person_character_glitch))

(fn ConstructionScript
  ;[0.9157 0.383 1] Create Material Instance and set render texture target
  (bind _returnvalue (Rendering|Material|CreateDynamicMaterialInstance "/Game/Materials/MI_Portal.MI_Portal" "None" "None" :!class /Script/Engine.KismetMaterialLibrary))
  (Rendering|Material|SetTextureParameterValue _returnvalue "RenderTexture" (Variables|Default|GetRender%20Target%20Texture))
  (Rendering|Material|SetMaterial (Variables|Default|GetPortal) 0 _returnvalue)
  (Variables|/Script/Engine.SceneCaptureComponent2D|SetTextureTarget (Variables|Default|GetPortalViewCapture) (Variables|BP_PortalDoor_C|GetRender%20Target%20Texture (Variables|Default|GetTeleport%20Target))))

(fn TeleportPlayer
  (params (Player :type BP%20First%20Person%20Character%20Glitch%20Object%20Reference))
  (bind _teleport_target (Variables|Default|GetTeleport%20Target))
  (bind _portalviewbackface (Variables|Default|GetPortalViewBackface))
  (bind _returnvalue (Transformation|GetWorldTransform _portalviewbackface))
  (bind _returnvalue_2 (Transformation|GetActorTransform _teleport_target))
  (bind _firstpersoncamera (Variables|/Game/Blueprints/Player/BP_FirstPersonCharacter_Glitch.BP_FirstPersonCharacter_Glitch_C|GetFirstPersonCamera Player))
  (bind _returnvalue_3 (Transformation|GetWorldTransform _firstpersoncamera))
  (bind _returnvalue_4 (Class|KismetMathLibrary|ConvertTransformtoRelative _returnvalue _returnvalue_3))
  (bind _returnvalue_5 (Math|Transform|ComposeTransforms _returnvalue_4 _returnvalue_2))
  (bind (_roll _pitch _yaw) (Math|Rotator|BreakRotator (.rotation _returnvalue_5)))
  (LocalVariables|SetRelativeVelocity (Math|Transform|InverseTransformDirection (Transformation|GetActorTransform Player) (Transformation|GetVelocity Player)))
  (Transformation|SetActorLocation Player (+ (* (Transformation|GetActorForwardVector (Variables|Default|GetTeleport%20Target)) -2.0) (Math|Vector|MakeVector (.x (.location _returnvalue_5)) (.y (.location _returnvalue_5)) (- (.z (.location _returnvalue_5)) 3e+01))) false false)
  (Pawn|SetControlRotation (Pawn|GetController Player) (Math|Rotator|MakeRotator 0.0 _pitch _yaw))
  (Variables|/Script/Engine.MovementComponent|SetVelocity (Pawn|GetMovementComponent Player) (Math|Transform|TransformDirection (Math|Transform|MakeTransform (Transformation|GetActorLocation Player) (Pawn|GetControlRotation (Pawn|GetController Player) :!class /Script/Engine.Controller)) (LocalVariables|GetRelativeVelocity))))